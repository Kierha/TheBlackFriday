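; BP_NPC is an NPC Blueprint that steps through an array of dialogue lines each time its Talk event fires.
; Talk increments the index first, then prints that line via PrintString if it is within the array.
; On such a valid line it also creates the WB_Dialog widget if none exists and adds it to the viewport, without passing it the text.
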(event `/Game/Dialogue/BPI_Dialog.Talk`
  (`/Engine/EditorBlueprintResources/StandardMacros.IncrementInt` (`self.DialogIndex`)
    (:`  `
      (if (< (`self.DialogIndex`) (`KismetArrayLibrary.Array_Length` (`self.Dialog`)))
        (`KismetSystemLibrary.PrintString` (`|GetArrayItem` (`self.Dialog`) (`self.DialogIndex`)))
        (`self.UI`
          (:`then`)
          (:`else`
            (bind _returnvalue (`|CreateWidget` "/Game/Dialogue/WB_Dialog.WB_Dialog_C" (`GameplayStatics.GetPlayerController` 0)))
            (bind _output_get (set `self.UI` _returnvalue))
            (`UserWidget.AddToViewport` _output_get 0)))))))

(fn `UserConstructionScript`)